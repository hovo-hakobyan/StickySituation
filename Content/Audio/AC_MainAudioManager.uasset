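; Audio manager, by its name an actor component, that plays sound cues on caller-supplied audio components for cooking and customer sounds.
; Cooking audio starts once through a DoOnce, with a looping timer feeding the CookingTime parameter every 0.1 seconds.
; Stopping halts the component, clears that timer by re-setting it at zero time and resets the DoOnce.
; Customer audio sets an integer CustomerState parameter before playing through the shared play event.
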(event `self.PlayAudio`
  (params (pSoundCue :type "SoundCue Object Reference") (pAudioComponent :type "AudioComponent Object Reference"))
  (`AudioComponent.SetSound` pAudioComponent pSoundCue)
  (`AudioComponent.Play` pAudioComponent 0.0))

(event `self.CookingAudio`
  (params (pSoundCue :type "SoundCue Object Reference") (pAudioComponent :type "AudioComponent Object Reference") (pCookingTime :type "Float (single-precision)"))
  (`/Engine/EditorBlueprintResources/StandardMacros.DoOnce` false :!label _label
    (:`Completed`
      (`self.PlayAudio` pSoundCue pAudioComponent)
      (`KismetSystemLibrary.K2_SetTimerDelegate` (delegate `SetCookingTIme`) 0.1 true))))

(event `SetCookingTIme`
  (`AudioParameterControllerInterface.SetFloatParameter` (stale `self.CookingAudio` pAudioComponent) "CookingTime" (stale `self.CookingAudio` pCookingTime)))

(event `self.StopAudio`
  (params (pAudioComponent :type "AudioComponent Object Reference"))
  (`AudioComponent.Stop` pAudioComponent)
  (`KismetSystemLibrary.K2_SetTimerDelegate` (delegate `SetCookingTIme`))
  (goto _label :!via `Reset`))

(event `self.CustomerAudio`
  (params (pSoundCue :type "SoundCue Object Reference") (pAudioComponent :type "AudioComponent Object Reference") (pcustomerState :type "CustomerState Enum (by ref)" :default "Happy"))
  (`AudioParameterControllerInterface.SetIntParameter` pAudioComponent "CustomerState" (`KismetMathLibrary.Conv_ByteToInt` pcustomerState))
  (`self.PlayAudio` pSoundCue pAudioComponent))
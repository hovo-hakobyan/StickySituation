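; BP_Customer is the customer character, which animates by state, reacts to dishes and slams the table.
; Tick does one-time setup linking AnimBP_Customer and a game pre-end flag, then pushes the current customer state to the AnimBP each frame.
; A table-slam callback spawns Niagara impacts at left and right smash points relative to the box component.
; Overlapping a Dish triggers chewing, and a separate event plays state-based idle audio through the main audio manager.
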(event `Play_CustomerAudio`
  (`AudioManager.CustomerAudio` (`self.AC_MainAudioManager`) "/Game/Audio/SoundCues/SFX/SC_CustomerIdle.SC_CustomerIdle" (`self.CustomerIdleAudioComponent`) (`self.currentCustomerState`)))

(event `self.ReceiveBeginPlay`)

(event `Reset`)

(event `self.ReceiveTick`
  (params (DeltaSeconds :type "Float (single-precision)"))
  (`|ExecutionSequence`
    (:`then_0`
      (`/Engine/EditorBlueprintResources/StandardMacros.DoOnce` false
        (:`Completed`
          (bind _asanim_bp_customer (cast `/Game/ArtAssets/Characters/Dragon/Anims/AnimBP_Customer` (`SkeletalMeshComponent.GetAnimInstance` (`self.SkeletalMesh`))))
          (bind _output_get (set `self.AnimBP` _asanim_bp_customer))
          (set `/Game/ArtAssets/Characters/Dragon/Anims/AnimBP_Customer.Customer` self _output_get)
          (add `self.OnGamePreEnd` (delegate `CustomEvent_0`)))))
    (:`then_1`
      (set `self.canTransition` true)
      (set `/Game/ArtAssets/Characters/Dragon/Anims/AnimBP_Customer.State` (`self.currentCustomerState`) (`self.AnimBP`))
      (add `/Game/ArtAssets/Characters/Dragon/Anims/AnimBP_Customer.SlamTable` (`self.AnimBP`) (delegate `SlamTable_Event_0`)))))

(event `CustomEvent_0`
  (set `/Game/ArtAssets/Characters/Dragon/Anims/AnimBP_Customer.GameEnd` true (stale `self.ReceiveTick` _output_get)))

(event `SlamTable_Event_0`
  (bind _boxcomponent (`self.BoxComponent`))
  (bind (_leftsmashlocation_x _leftsmashlocation_y _leftsmashlocation_z) (`KismetMathLibrary.BreakVector` (`self.LeftSmashLocation`)))
  (bind _boxcomponent_2 (`self.BoxComponent`))
  (bind (_rightsmashlocation_x _rightsmashlocation_y _rightsmashlocation_z) (`KismetMathLibrary.BreakVector` (`self.RightSmashLocation`)))
  (`NiagaraFunctionLibrary.SpawnSystemAtLocation` "/Game/RFX/Emitters/Impact_Simple_NS.Impact_Simple_NS" (+ (* (`KismetMathLibrary.MakeVector` (* _leftsmashlocation_y -1.0) (* _leftsmashlocation_x -1.0) _leftsmashlocation_z) (`SceneComponent.RelativeScale3D` _boxcomponent_2)) (`SceneComponent.K2_GetComponentLocation` _boxcomponent_2)))
  (`NiagaraFunctionLibrary.SpawnSystemAtLocation` "/Game/RFX/Emitters/Impact_Simple_NS.Impact_Simple_NS" (+ (* (`KismetMathLibrary.MakeVector` (* _rightsmashlocation_y -1.0) (* _rightsmashlocation_x -1.0) _rightsmashlocation_z) (`SceneComponent.RelativeScale3D` _boxcomponent)) (`SceneComponent.K2_GetComponentLocation` _boxcomponent))))

(event `self.BoxComponent.OnComponentBeginOverlap`
  (params (OverlappedComponent :type "PrimitiveComponent Object Reference") (OtherActor :type "Actor Object Reference") (OtherComp :type "PrimitiveComponent Object Reference") (OtherBodyIndex :type Integer) (bFromSweep :type Boolean) (SweepResult :type "HitResult Structure (by ref)"))
  (if (`KismetMathLibrary.ClassIsChildOf` (`GameplayStatics.GetObjectClass` OtherActor) "/Script/StickySituation.Dish")
    (set `/Game/ArtAssets/Characters/Dragon/Anims/AnimBP_Customer.Is Chewing` true (`self.AnimBP`))))

(fn `UserConstructionScript`)
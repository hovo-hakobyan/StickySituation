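; Grill interactable that shows fire effects while switched on and can flash its material.
; Tick polls IsGrillOn through a redundant self-cast and activates or deactivates four fire effect components every frame.
; When ShouldFlash is set, a DoOnce fires StartFlashing, which sets a scalar material parameter on VisibleComponent.
; StopFlashing clears that parameter, but its only call here is unwired, so this graph never stops the flashing.
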(event `Start Flashing`
  ;[1 1 1] Flashing of material
  (`MeshComponent.SetScalarParameterValueOnMaterials` (`self.VisibleComponent`) "IsFlashing?" 1.0))

(event `Stop Flashing`
  ;[1 1 1] Flashing of material
  (`MeshComponent.SetScalarParameterValueOnMaterials` (`self.VisibleComponent`) "IsFlashing?" 0.0))

(event `self.ReceiveBeginPlay`)

(event `self.ReceiveTick`
  (params (DeltaSeconds :type "Float (single-precision)"))
  ;[1 1 1] Cast, otherwise getting is not posible.
  (bind _asbp_gril (cast `/Game/Blueprints/Gameplay/Interactables/BP_Gril` self))
  (`|ExecutionSequence`
    (:`then_0`
      (if (`Grill.bIsGrillOn` _asbp_gril)
        (`ActorComponent.Activate` (`self.Fire_NS3`) false)
        (`ActorComponent.Activate` (`self.Fire_NS2`) false)
        (`ActorComponent.Activate` (`self.Fire_NS1`) false)
        (`ActorComponent.Activate` (`self.Fire_NS`) false)
        (else
          (`ActorComponent.Deactivate` (`self.Fire_NS`))
          (`ActorComponent.Deactivate` (`self.Fire_NS1`))
          (`ActorComponent.Deactivate` (`self.Fire_NS2`))
          (`ActorComponent.Deactivate` (`self.Fire_NS3`)))))
    (:`then_1`
      (if (`self.bShouldFlash`)
        (`/Engine/EditorBlueprintResources/StandardMacros.DoOnce` false
          (:`Completed`
            (`self.Start Flashing`)))))))

(fn `UserConstructionScript`)
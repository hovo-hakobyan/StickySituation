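; BP_Keypad is an in-world virtual keyboard actor for entering the team name.
; It starts hidden, then appears with collision and a viewport overlay when the camera manager's keyboard look ends, if the game mode allows it.
; Enter saves non-empty text from the linked display to the game mode, flags the camera toward the main game and hides both actors' interfaces.
; The camera delegate binds through a DoOnce on Tick rather than BeginPlay.
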(event `self.ReceiveBeginPlay`
  (bind _asbp_main_game_mode (cast `/Game/Blueprints/Gameplay/GameModes/BP_MainGameMode` (`GameplayStatics.GetGameMode`)))
  (set `self.GameModeREF` _asbp_main_game_mode)
  (bind _aswbp_keypad (cast `/Game/Blueprints/UI/WBP_Keypad` (`WidgetComponent.GetUserWidgetObject` (`self.Keypad Widget`))))
  (add `/Game/Blueprints/UI/WBP_Keypad.EnterPress` _aswbp_keypad (delegate `EnterPress_Event_0`))
  (bind _returnvalue (`|CreateWidget` "/Game/Blueprints/UI/WBP_KeypadOverlay.WBP_KeypadOverlay_C" (`GameplayStatics.GetPlayerController` 0)))
  (set `self.KeypadOverlay` _returnvalue)
  (`self.HideKeyboard`))

(event `EnterPress_Event_0`
  (bind _finaltext (`self.FinalText`))
  (bind _gamemoderef (`self.GameModeREF`))
  (bind _aswbp_keypad_display (cast `/Game/Blueprints/UI/WBP_KeypadDisplay` (`WidgetComponent.GetUserWidgetObject` (`/Game/Blueprints/Gameplay/Interactables/BP_KeypadDisplay.Keypad Display Widget` (`self.TargetDisplay`)))))
  (set `self.FinalText` (`EditableTextBox.GetText` (`/Game/Blueprints/UI/WBP_KeypadDisplay.EditableTextBox_41` _aswbp_keypad_display)))
  (if (not (`KismetTextLibrary.TextIsEmpty` _finaltext))
    (set `StickySituationGameModeBase.CurrentTeamName` (`KismetTextLibrary.Conv_TextToString` _finaltext) _gamemoderef)
    (set `CameraManager.bShouldLookAtMainGame` true (`StickySituationGameModeBase.CameraManager` _gamemoderef))
    (`self.HideKeyboard`)
    (`/Game/Blueprints/Gameplay/Interactables/BP_KeypadDisplay.HideKeypadDisplay` (`self.TargetDisplay`))))

(event `self.ReceiveTick`
  (params (DeltaSeconds :type "Float (single-precision)"))
  (`/Engine/EditorBlueprintResources/StandardMacros.DoOnce` false
    (:`Completed`
      (add `CameraManager.CameraEndsLookingAtKeyboard` (`StickySituationGameModeBase.CameraManager` (`self.GameModeREF`)) (delegate `CameraEndsLookingAtKeyboard_Event_0`)))))

(event `CameraEndsLookingAtKeyboard_Event_0`
  (if (`StickySituationGameModeBase.ShouldDisplayVirtualKeyboard` (`self.GameModeREF`))
    (`self.ShowKeyboard`)))

(event `ShowKeyboard`
  (`self.SetActorHiddenInGame` false)
  (`self.SetActorEnableCollision` true)
  ;[1 1 1] Show the overlay widget here
  (`UserWidget.AddToViewport` (`self.KeypadOverlay`) 0))

(event `HideKeyboard`
  (`self.SetActorHiddenInGame` true)
  (`self.SetActorEnableCollision` false)
  ;[1 1 1] Hide the overlay widget here
  (`Widget.RemoveFromParent` (`self.KeypadOverlay`)))

(fn `UserConstructionScript`)
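; BP_KeypadDisplay is an interactable actor that shows a virtual keypad display once the camera has settled on the in-game keyboard.
; It starts hidden with collision off, and on its first tick binds to the game mode camera manager's event for ending a look at the keyboard.
; That event reveals the display if the game mode allows a virtual keyboard, then a delayed WidgetInteraction left-click focuses the textbox.
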(event `self.ReceiveBeginPlay`
  (bind _asbp_main_game_mode (cast `/Game/Blueprints/Gameplay/GameModes/BP_MainGameMode` (`GameplayStatics.GetGameMode`)))
  (set `self.GameModeREF` _asbp_main_game_mode)
  (`self.HideKeypadDisplay`))

(event `self.ReceiveTick`
  (params (DeltaSeconds :type "Float (single-precision)"))
  (`/Engine/EditorBlueprintResources/StandardMacros.DoOnce` false
    (:`Completed`
      (add `CameraManager.CameraEndsLookingAtKeyboard` (`StickySituationGameModeBase.CameraManager` (`self.GameModeREF`)) (delegate `CameraEndsLookingAtKeyboard_Event_0`)))))

(event `CameraEndsLookingAtKeyboard_Event_0`
  (if (`StickySituationGameModeBase.ShouldDisplayVirtualKeyboard` (`self.GameModeREF`))
    (`self.ShowKeypadDisplay`)))

(event `ShowKeypadDisplay`
  (`self.SetActorHiddenInGame` false)
  (`self.SetActorEnableCollision` true)
  ;[1 1 1] Focus the textbox
  (`KismetSystemLibrary.Delay` 0.5)
  (`WidgetInteractionComponent.PressPointerKey` (`self.WidgetInteraction`) "LeftMouseButton"))

(event `HideKeypadDisplay`
  (`self.SetActorHiddenInGame` true)
  (`self.SetActorEnableCollision` false))

(fn `UserConstructionScript`)
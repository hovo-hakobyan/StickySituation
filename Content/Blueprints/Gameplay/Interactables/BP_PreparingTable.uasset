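; Preparing table interactable with a bell button, where dishes are prepared and feedback is given through sound, particles and a flashing material.
; When a chopstick pawn overlaps the button, it rings the bell and, after a short delay, spawns a cross Niagara effect if no Dish actor exists.
; Any button overlap also binds the dish-prepared sound to OnDishPrepare.
; Start and stop events toggle flashing through a material scalar parameter.
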(event `self.StartFlashing`
  ;[1 1 1] Flashing of material
  (`MeshComponent.SetScalarParameterValueOnMaterials` (`self.VisibleComponent`) "IsFlashing?" 1.0)
  (set `self.bHasFlashed` true))

(event `self.ReceiveTick`
  (params (DeltaSeconds :type "Float (single-precision)")))

(event `self.StopFlashing`
  ;[1 1 1] Flashing of material
  (`MeshComponent.SetScalarParameterValueOnMaterials` (`self.VisibleComponent`) "IsFlashing?" 0.0))

(event `self.ReceiveBeginPlay`)

(event `self.ButtonCollisionComponent.OnComponentBeginOverlap`
  (params (OverlappedComponent :type "PrimitiveComponent Object Reference") (OtherActor :type "Actor Object Reference") (OtherComp :type "PrimitiveComponent Object Reference") (OtherBodyIndex :type Integer) (bFromSweep :type Boolean) (SweepResult :type "HitResult Structure (by ref)"))
  (bind _collisioncomponent (`self.CollisionComponent`))
  (bind (_crossparticle_location_x _crossparticle_location_y _crossparticle_location_z) (`KismetMathLibrary.BreakVector` (`self.CrossParticle_Location`)))
  (`|ExecutionSequence`
    (:`then_0`
      (cast `/Game/Blueprints/Gameplay/Pawns/BP_ChopstickPawn` OtherActor)
      (`AudioManager.PlayAudio` (`self.AC_MainAudioManager`) "/Game/Audio/SoundCues/SFX/SC_Bell.SC_Bell" (`self.BellAudioComponent`))
      (`KismetSystemLibrary.Delay` 0.1)
      (bind _outactors (`GameplayStatics.GetAllActorsOfClass` "/Script/StickySituation.Dish"))
      (if (== (`KismetArrayLibrary.Array_Length` _outactors) 0)
        (`NiagaraFunctionLibrary.SpawnSystemAtLocation` "/Game/RFX/Emitters/Cross_NS.Cross_NS" (+ (* (`KismetMathLibrary.MakeVector` (* _crossparticle_location_y -1.0) (* _crossparticle_location_x -1.0) _crossparticle_location_z) (`SceneComponent.RelativeScale3D` _collisioncomponent)) (`SceneComponent.K2_GetComponentLocation` _collisioncomponent)))))
    (:`then_1`
      (add `self.OnDishPrepare` self (delegate `Play_PrepareAudio`)))))

(event `Play_PrepareAudio`
  (`AudioManager.PlayAudio` (`self.AC_MainAudioManager`) "/Game/Audio/SoundCues/SFX/SC_DishPrepared.SC_DishPrepared" (`self.PrepareAudioComponent`)))

(fn `UserConstructionScript`)
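; BP_SelectionScreen is an in-world menu actor with a selection widget offering change-name and start-game actions.
; It starts hidden and appears with the keypad controls overlay when the camera finishes looking at the keyboard, unless the virtual keyboard should display.
; Changing name hides it and shows the keypad and its display; starting hides it and points the camera manager at the main game.
; The camera callback is bound once from Tick through DoOnce.
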(event `StartGame`
  (set `CameraManager.bShouldLookAtMainGame` true (`StickySituationGameModeBase.CameraManager` (`self.GameModeREF`)))
  (`self.HideSelectionScreen`))

(event `self.ReceiveBeginPlay`
  (bind _aswbp_selection (cast `/Game/Blueprints/UI/WBP_Selection` (`WidgetComponent.GetUserWidgetObject` (`self.Widget`))))
  (add `/Game/Blueprints/UI/WBP_Selection.ChangeName` _aswbp_selection (delegate `ChangeName`))
  (add `/Game/Blueprints/UI/WBP_Selection.StartGame` _aswbp_selection (delegate `StartGame`))
  (bind _asbp_main_game_mode (cast `/Game/Blueprints/Gameplay/GameModes/BP_MainGameMode` (`GameplayStatics.GetGameMode`)))
  (set `self.GameModeREF` _asbp_main_game_mode)
  (bind _returnvalue (`|CreateWidget` "/Game/Blueprints/UI/WBP_KeypadOverlay.WBP_KeypadOverlay_C" (`GameplayStatics.GetPlayerController` 0)))
  (set `self.Keypad Overlay` _returnvalue)
  (`self.HideSelectionScreen`))

(event `ChangeName`
  (`self.HideSelectionScreen`)
  (bind _returnvalue (`GameplayStatics.GetActorOfClass` "/Game/Blueprints/Gameplay/Interactables/BP_Keypad.BP_Keypad_C"))
  (`/Game/Blueprints/Gameplay/Interactables/BP_Keypad.ShowKeyboard` _returnvalue)
  (bind _returnvalue_2 (`GameplayStatics.GetActorOfClass` "/Game/Blueprints/Gameplay/Interactables/BP_KeypadDisplay.BP_KeypadDisplay_C"))
  (`/Game/Blueprints/Gameplay/Interactables/BP_KeypadDisplay.ShowKeypadDisplay` _returnvalue_2))

(event `self.ReceiveTick`
  (params (DeltaSeconds :type "Float (single-precision)"))
  (`/Engine/EditorBlueprintResources/StandardMacros.DoOnce` false
    (:`Completed`
      (add `CameraManager.CameraEndsLookingAtKeyboard` (`StickySituationGameModeBase.CameraManager` (`self.GameModeREF`)) (delegate `CustomEvent_0`)))))

(event `CustomEvent_0`
  (if (not (`StickySituationGameModeBase.ShouldDisplayVirtualKeyboard` (`self.GameModeREF`)))
    (`self.ShowSelectionScreen`)))

(event `HideSelectionScreen`
  (`self.SetActorHiddenInGame` true)
  (`self.SetActorEnableCollision` false)
  ;[1 1 1] Hide controls widget here
  (`Widget.RemoveFromParent` (`self.Keypad Overlay`)))

(event `ShowSelectionScreen`
  (`self.SetActorHiddenInGame` false)
  (`self.SetActorEnableCollision` true)
  ;[1 1 1] Show controls widget here
  (`UserWidget.AddToViewport` (`self.Keypad Overlay`) 0))

(fn `UserConstructionScript`)
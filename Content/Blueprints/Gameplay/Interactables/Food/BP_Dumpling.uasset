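; BP_Dumpling is a food interactable that spawns a poof effect on BeginPlay and drives a material bounce when hit.
; Collision hits write the impact location to the M_BounceParameters collection, while a timeline animates the impact normal scaled by StrengthBounces.
; Every hit resets a debounce timer, so only hits following a quiet interval restart the bounce.
; The parameter collection is shared, so dumplings overwrite each other's bounce values.
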(event `self.ReceiveBeginPlay`
  (set `self.Time` 0.0)
  (`NiagaraFunctionLibrary.SpawnSystemAtLocation` "/Game/RFX/Emitters/Poof_NS.Poof_NS" (`SceneComponent.K2_GetComponentLocation` (`self.VisibleComponent`))))

(event `self.CollisionComponent.OnComponentHit`
  (params (HitComponent :type "PrimitiveComponent Object Reference") (OtherActor :type "Actor Object Reference") (OtherComp :type "PrimitiveComponent Object Reference") (NormalImpulse :type "Vector Structure") (Hit :type "HitResult Structure (by ref)"))
  (bind (_bblockinghit _binitialoverlap _time _distance _location _impactpoint _normal _impactnormal) (`GameplayStatics.BreakHitResult` Hit))
  (bind _returnvalue (`KismetSystemLibrary.GetGameTimeInSeconds`))
  ;[1 1 1] Time between hits (so they dont trigger in quick sucession
  (if (< (- _returnvalue (`self.Time`)) (`self.Time between registering hits`))
    (set `self.Time` _returnvalue)
    (else
      (set `self.Time` _returnvalue)
      (`KismetMaterialLibrary.SetVectorParameterValue` "/Game/BaseMaterials/M_BounceParameters.M_BounceParameters" "Location" (`KismetMathLibrary.Conv_VectorToLinearColor` _location))
      (bind (_direction _newtrack_0) (`Timeline|Timeline_0` :!via `PlayFromStart`)
        (:`Update`
          (`KismetMaterialLibrary.SetVectorParameterValue` "/Game/BaseMaterials/M_BounceParameters.M_BounceParameters" "Normal" (`KismetMathLibrary.Conv_VectorToLinearColor` (* _impactnormal (* _newtrack_0 (`self.Strength Bounces`))))))))))

(fn `UserConstructionScript`)
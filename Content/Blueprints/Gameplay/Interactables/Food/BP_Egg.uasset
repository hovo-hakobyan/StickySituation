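; BP_Egg is a cookable egg ingredient that breaks when it hits something after falling.
; Tick spawns one-time cooked or burned effects and arms breaking once the fall lasts long enough.
; Hitting actors not tagged DynamicObject or Interactable copies cooking blend values to a Material Parameter Collection, spawns a broken-egg effect and destroys the egg.
; Overlapping BP_GroundToCollide spawns a splash.
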(event `self.ReceiveTick`
  (params (DeltaSeconds :type "Float (single-precision)"))
  (bind (_returnvalue_x _returnvalue_y _returnvalue_z) (`KismetMathLibrary.BreakVector` (`self.GetVelocity`)))
  (bind _visiblecomponent (`self.VisibleComponent`))
  (`|ExecutionSequence`
    (:`then_0`
      (bind _returnvalue (`self.GetIngredientState`))
      (switch `EFoodState` _returnvalue
        (:`Cooked`
          (`/Engine/EditorBlueprintResources/StandardMacros.DoOnce` false
            (:`Completed`
              (`NiagaraFunctionLibrary.SpawnSystemAtLocation` "/Game/RFX/Emitters/Sparkle_NS.Sparkle_NS" (`SceneComponent.K2_GetComponentLocation` _visiblecomponent)))))
        (:`Burned`
          (`/Engine/EditorBlueprintResources/StandardMacros.DoOnce` false
            (:`Completed`
              (`NiagaraFunctionLibrary.SpawnSystemAtLocation` "/Game/RFX/Emitters/Food_Burned_NS.Food_Burned_NS" (`SceneComponent.K2_GetComponentLocation` _visiblecomponent)))))))
    (:`then_1`
      (if (<= _returnvalue_z -5.0)
        (set `self.CurrentBreakTime` (+ DeltaSeconds (`self.CurrentBreakTime`)))
        (if (>= (`self.CurrentBreakTime`) (`self.BreakAfterSeconds`))
          (set `self.bCanBreak` true))
        (else
          (set `self.CurrentBreakTime` 0.0))))))

(event `self.CollisionComponent.OnComponentHit`
  (params (HitComponent :type "PrimitiveComponent Object Reference") (OtherActor :type "Actor Object Reference") (OtherComp :type "PrimitiveComponent Object Reference") (NormalImpulse :type "Vector Structure") (Hit :type "HitResult Structure (by ref)"))
  (if (or (`self.ActorHasTag` OtherActor "DynamicObject") (`self.ActorHasTag` OtherActor "Interactable"))
    _
    (elif (`self.bCanBreak`)
      (`/Engine/EditorBlueprintResources/StandardMacros.DoOnce` false
        (:`Completed`
          (bind _returnvalue (`PrimitiveComponent.CreateDynamicMaterialInstance` (`self.VisibleComponent`) 0 null "None"))
          (set `self.Eggo` _returnvalue)
          (`self.Set MaterialsToFollowCooking`)
          (`NiagaraFunctionLibrary.SpawnSystemAtLocation` (`self.BrokenEgg`) (`SceneComponent.K2_GetComponentLocation` (`self.CollisionComponent`)) (struct) (1.0 1.0 1.0) false)
          (`self.K2_DestroyActor`))))))

(event `self.CollisionComponent.OnComponentBeginOverlap`
  (params (OverlappedComponent :type "PrimitiveComponent Object Reference") (OtherActor :type "Actor Object Reference") (OtherComp :type "PrimitiveComponent Object Reference") (OtherBodyIndex :type Integer) (bFromSweep :type Boolean) (SweepResult :type "HitResult Structure (by ref)"))
  (cast `/Game/Blueprints/Gameplay/Interactables/BP_GroundToCollide` OtherActor)
  (`NiagaraFunctionLibrary.SpawnSystemAtLocation` "/Game/RFX/Emitters/Splash_NS.Splash_NS" (`SceneComponent.K2_GetComponentLocation` (`self.CollisionComponent`))))

(fn `Set MaterialsToFollowCooking`
  (bind _eggo (`self.Eggo`))
  (bind _returnvalue (`MaterialInstanceDynamic.K2_GetScalarParameterValue` _eggo "Blend Value Burnt"))
  (`KismetMaterialLibrary.SetScalarParameterValue` "/Game/ArtAssets/Props/Egg/Materials/MPC_EggYolkCooking.MPC_EggYolkCooking" "Blend Value Burnt" _returnvalue)
  (bind _returnvalue_2 (`MaterialInstanceDynamic.K2_GetScalarParameterValue` _eggo "Blend Value Cooked"))
  (`KismetMaterialLibrary.SetScalarParameterValue` "/Game/ArtAssets/Props/Egg/Materials/MPC_EggYolkCooking.MPC_EggYolkCooking" "Blend Value Cooked" _returnvalue_2)
  (bind _returnvalue_3 (`MaterialInstanceDynamic.K2_GetScalarParameterValue` _eggo "Blend Value Cooking"))
  (`KismetMaterialLibrary.SetScalarParameterValue` "/Game/ArtAssets/Props/Egg/Materials/MPC_EggYolkCooking.MPC_EggYolkCooking" "Blend Value Cooking" _returnvalue_3))

(fn `UserConstructionScript`)
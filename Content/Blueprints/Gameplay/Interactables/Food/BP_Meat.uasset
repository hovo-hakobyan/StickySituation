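; BP_Meat is a food ingredient interactable that gives visual feedback as it cooks and when it hits the ground.
; Each tick it checks its ingredient state and, through one-shot gates, spawns a sparkle Niagara effect at the visible mesh when Cooked or a burned effect when Burned.
; Overlapping a BP_GroundToCollide actor with its collision component spawns a splash effect at that spot.
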(event `self.ReceiveTick`
  (params (DeltaSeconds :type "Float (single-precision)"))
  (bind _visiblecomponent (`self.VisibleComponent`))
  (bind _returnvalue (`self.GetIngredientState`))
  (switch `EFoodState` _returnvalue
    (:`Cooked`
      (`/Engine/EditorBlueprintResources/StandardMacros.DoOnce` false
        (:`Completed`
          (`NiagaraFunctionLibrary.SpawnSystemAtLocation` "/Game/RFX/Emitters/Sparkle_NS.Sparkle_NS" (`SceneComponent.K2_GetComponentLocation` _visiblecomponent)))))
    (:`Burned`
      (`/Engine/EditorBlueprintResources/StandardMacros.DoOnce` false
        (:`Completed`
          (`NiagaraFunctionLibrary.SpawnSystemAtLocation` "/Game/RFX/Emitters/Food_Burned_NS.Food_Burned_NS" (`SceneComponent.K2_GetComponentLocation` _visiblecomponent)))))))

(event `self.CollisionComponent.OnComponentBeginOverlap`
  (params (OverlappedComponent :type "PrimitiveComponent Object Reference") (OtherActor :type "Actor Object Reference") (OtherComp :type "PrimitiveComponent Object Reference") (OtherBodyIndex :type Integer) (bFromSweep :type Boolean) (SweepResult :type "HitResult Structure (by ref)"))
  (cast `/Game/Blueprints/Gameplay/Interactables/BP_GroundToCollide` OtherActor)
  (`NiagaraFunctionLibrary.SpawnSystemAtLocation` "/Game/RFX/Emitters/Splash_NS.Splash_NS" (`SceneComponent.K2_GetComponentLocation` (`self.CollisionComponent`))))

(fn `UserConstructionScript`)
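; Chopstick pawn that presses a world-space keypad through a widget interaction component and spawns a bell particle on touching the PreparingTable's button.
; A downward trace each tick sets the shadow blob decal's opacity by hit distance as a depth cue.
; Tick also toggles the mesh's Fresnel material parameter by game mode state, requesting a dynamic material instance each frame.
; Keypad presses and releases trim the display text to MaxCharacters.
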(event `self.ReceiveBeginPlay`
  (bind _returnvalue (`KismetMaterialLibrary.CreateDynamicMaterialInstance` "/Game/BaseMaterials/MI_ShadowBlob.MI_ShadowBlob"))
  (bind _output_get (set `self.DynamicDecalMaterial` _returnvalue))
  (`DecalComponent.SetDecalMaterial` (`self.Decal`) _output_get)
  (`MaterialInstanceDynamic.SetScalarParameterValue` _output_get "Opacity" 0.8)
  (bind _returnvalue_2 (`GameplayStatics.GetActorOfClass` "/Game/Blueprints/Gameplay/Interactables/BP_Keypad.BP_Keypad_C"))
  (bind _aswbp_keypad (cast `/Game/Blueprints/UI/WBP_Keypad` (`WidgetComponent.GetUserWidgetObject` (`/Game/Blueprints/Gameplay/Interactables/BP_Keypad.Keypad Widget` _returnvalue_2))))
  (set `self.KeypadWidget` _aswbp_keypad)
  (bind _returnvalue_3 (`GameplayStatics.GetActorOfClass` "/Game/Blueprints/Gameplay/Interactables/BP_KeypadDisplay.BP_KeypadDisplay_C"))
  (bind _aswbp_keypad_display (cast `/Game/Blueprints/UI/WBP_KeypadDisplay` (`WidgetComponent.GetUserWidgetObject` (`/Game/Blueprints/Gameplay/Interactables/BP_KeypadDisplay.Keypad Display Widget` _returnvalue_3))))
  (set `self.KeypadDisplayWidget` _aswbp_keypad_display))

(event `self.ReceiveTick`
  (params (DeltaSeconds :type "Float (single-precision)"))
  (bind _returnvalue (`self.K2_GetActorLocation`))
  (bind _visiblecomponent (`self.VisibleComponent`))
  (`|ExecutionSequence`
    (:`then_0`
      (bind (_outhit _returnvalue_2) (`KismetSystemLibrary.LineTraceSingle` _returnvalue (- _returnvalue (0.0 0.0 10000.0)) "TraceTypeQuery1"))
      (if _returnvalue_2
        (`MaterialInstanceDynamic.SetScalarParameterValue` (`self.DynamicDecalMaterial`) "Opacity" (`KismetMathLibrary.Lerp` 0.9 0.4 (`.Time` (`GameplayStatics.BreakHitResult` _outhit))))
        (`SceneComponent.K2_SetWorldRotation` (`self.Decal`) (`KismetMathLibrary.MakeRotator` 0.0 90.0) false false)))
    (:`then_1`
      (bind _asbp_main_game_mode (cast `/Game/Blueprints/Gameplay/GameModes/BP_MainGameMode` (`GameplayStatics.GetGameMode`)))
      (if (`|EnumEquality` (`StickySituationGameModeBase.CurrentGameState` _asbp_main_game_mode) "GameplayState")
        (bind _returnvalue_3 (`PrimitiveComponent.CreateDynamicMaterialInstance` _visiblecomponent 0 null "None"))
        (`MaterialInstanceDynamic.SetScalarParameterValue` _returnvalue_3 "Fresnel BC" 1.0)
        (else
          (bind _returnvalue_4 (`PrimitiveComponent.CreateDynamicMaterialInstance` _visiblecomponent 0 null "None"))
          (`MaterialInstanceDynamic.SetScalarParameterValue` _returnvalue_4 "Fresnel BC" 0.0))))))

(event `InputAction|VirtualKeyboardAction`
  (params (Key :type "Key Structure"))
  (bind _maxcharacters (`self.MaxCharacters`))
  (bind _widgetinteractioncomponent (`self.WidgetInteractionComponent`))
  (bind _editabletextbox_41 (`/Game/Blueprints/UI/WBP_KeypadDisplay.EditableTextBox_41` (`self.KeypadDisplayWidget`)))
  (bind _returnvalue (`KismetTextLibrary.Conv_TextToString` (`EditableTextBox.GetText` _editabletextbox_41)))
  (:`Pressed`
    (set `/Game/Blueprints/UI/WBP_Keypad.WidgetInteraction` (`self.WidgetInteractionComponent`) (`self.KeypadWidget`))
    (`WidgetInteractionComponent.PressPointerKey` _widgetinteractioncomponent "LeftMouseButton")
    (if (> (`KismetStringLibrary.Len` _returnvalue) _maxcharacters) :!label _label
      ;[1 1 1] Remove the last character
      (`EditableTextBox.SetText` _editabletextbox_41 (`KismetTextLibrary.Conv_StringToText` (`KismetStringLibrary.GetSubstring` _returnvalue 0 _maxcharacters)))))
  (:`Released`
    (`WidgetInteractionComponent.ReleasePointerKey` _widgetinteractioncomponent "LeftMouseButton")
    (goto _label)))

(event `self.CapsuleComponent.OnComponentBeginOverlap`
  (params (OverlappedComponent :type "PrimitiveComponent Object Reference") (OtherActor :type "Actor Object Reference") (OtherComp :type "PrimitiveComponent Object Reference") (OtherBodyIndex :type Integer) (bFromSweep :type Boolean) (SweepResult :type "HitResult Structure (by ref)"))
  ;[1 0.7266 0.3475] When Chopstick Touches the Bell, Bell Particle spawns
  (bind _aspreparing_table (cast `PreparingTable` OtherActor))
  (bind _buttoncollisioncomponent (`PreparingTable.ButtonCollisionComponent` _aspreparing_table))
  (if (`PrimitiveComponent.IsOverlappingComponent` _buttoncollisioncomponent (`self.CapsuleComponent`))
    (`NiagaraFunctionLibrary.SpawnSystemAtLocation` "/Game/RFX/Emitters/Bell_NS.Bell_NS" (`SceneComponent.K2_GetComponentLocation` _buttoncollisioncomponent))))

(fn `UserConstructionScript`)